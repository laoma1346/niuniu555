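; BP_TestDummy is a test target that takes hits and exposes health, defense and resistance queries.
; TakeDamage subtracts raw hit damage without applying defense or resistance, prints a Chinese debug message, passes the hit to HitReaction, and destroys the actor at zero health.
; Heal and GetHitReactionType are stubs, CanBeDamaged is always true, and GetResistance returns physical resistance for every damage type.
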(event `self.ReceiveBeginPlay`)

(fn `CanBeDamaged`
  (returns (ReturnValue :type Boolean))
  (return true))

(fn `GetCurrentHealth`
  (returns (ReturnValue :type "Float (single-precision)"))
  (return (`self.CurrentHealth`)))

(fn `GetDefense`
  (returns (ReturnValue :type "Float (single-precision)"))
  (return (`self.Defense`)))

(fn `GetHealthPercent`
  (returns (ReturnValue :type "Float (single-precision)"))
  (return (/ (`self.CurrentHealth`) (`self.MaxHealth`))))

(fn `GetHitReactionType`
  (params (Damage :type "Float (single-precision)") (KnockbackForce :type "Float (single-precision)"))
  (returns (ReturnValue :type "EHitReactionType Enum"))
  (return "None"))

(fn `GetMaxHealth`
  (returns (ReturnValue :type "Float (single-precision)"))
  (return (`self.MaxHealth`)))

(fn `GetResistance`
  (params (DamageType :type "EDamageType Enum" :default "Physical"))
  (returns (ReturnValue :type "Float (single-precision)"))
  (return (`self.PhysicalResistance`)))

(fn `Heal`
  (params (Amount :type "Float (single-precision)"))
  (returns (ReturnValue :type "Float (single-precision)"))
  (return 0.0))

(fn `IsAlive`
  (returns (ReturnValue :type Boolean))
  (return (> (`self.CurrentHealth`) 0.0)))

(fn `TakeDamage`
  (params (HitInfo :type "HitInfo Structure (by ref)"))
  (returns (ReturnValue :type "Float (single-precision)"))
  (bind (_damage _bcritical) (break `HitInfo` HitInfo))
  (bind _output_get (set `self.CurrentHealth` (- (`self.CurrentHealth`) _damage)))
  (`KismetSystemLibrary.PrintString` (`KismetTextLibrary.Conv_TextToString` (`|FormatText` "受到伤害: {Damage}, 暴击: {Critical}, 剩余生命: {CurrentHealth}" _damage _bcritical _output_get)))
  (`HitReactionComponent.ProcessHitReaction` (`self.HitReaction`) HitInfo)
  (if (<= _output_get 0.0)
    (`self.K2_DestroyActor`))
  (return _damage))

(fn `UserConstructionScript`)